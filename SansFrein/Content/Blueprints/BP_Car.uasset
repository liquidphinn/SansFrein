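; BP_Car is a physics-driven car that rides on raycast suspension at four corner booster components.
; Every Tick, SuspensionCast traces down from each booster and pushes the Box body along the trace's reverse direction at that point, scaling linearly with compression.
; The spring force has no damping term, and the traces draw debug lines for one frame.
; Tick also starts a world-space camera shake on the first player controller every frame.
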(event `self.ReceiveBeginPlay`)

(event `self.ReceiveTick`
  (params (DeltaSeconds :type "Float (single-precision)"))
  (`self.SuspensionCast` (`self.FL_Booster`))
  (`self.SuspensionCast` (`self.FR_Booster`))
  (`self.SuspensionCast` (`self.BR_Booster`))
  (`self.SuspensionCast` (`self.BL_Booster`))
  (`PlayerController.ClientStartCameraShake` :`self` (`GameplayStatics.GetPlayerController` 0) :`Shake` "/Game/Blueprints/Shake.Shake_C" :`PlaySpace` "World"))

(fn `SuspensionCast`
  (params (`Wheel Comp` :type "SceneComponent Object Reference"))
  (bind _returnvalue (`SceneComponent.K2_GetComponentLocation` `Wheel Comp`))
  (bind _outhit (`KismetSystemLibrary.LineTraceSingle` :`Start` _returnvalue :`End` (+ _returnvalue (* (`SceneComponent.GetUpVector` `Wheel Comp`) -60.0)) :`TraceChannel` "TraceTypeQuery1" :`DrawDebugType` "ForOneFrame"))
  (bind (_bblockinghit _binitialoverlap _time _distance _location _impactpoint _normal _impactnormal _physmat _hitactor _hitcomponent _hitbonename _bonename _hititem _elementindex _faceindex _tracestart _traceend) (`GameplayStatics.BreakHitResult` _outhit))
  (if _bblockinghit
    (`PrimitiveComponent.AddForceAtLocation` (`self.Box`) (* (- 1.0 (`KismetMathLibrary.NormalizeToRange` _distance 0.0 60.0)) (`KismetMathLibrary.GetDirectionUnitVector` _traceend _tracestart) 100000.0) (`SceneComponent.K2_GetComponentLocation` (`local.Wheel Comp`)) "None")))

(fn `UserConstructionScript`)