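; Camera pawn for a gun-themed, click-driven scene that creates the HUD on BeginPlay and keeps a score through an AddScore event.
; Left click plays a world camera shake at the pawn and traces under the cursor on Visibility, but nothing acts on the hit result.
; A small explosion effect spawn at the camera is left unconnected, and the overlap, tick and construction logic are empty.
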(event `AddScore`
  (params (Score :type Integer))
  ; Add Score To Player
  (set `self.Score` (+ Score (`self.Score`))))

(event `self.ReceiveBeginPlay`
  (bind _returnvalue (`|CreateWidget` "/Game/HUD.HUD_C"))
  (`UserWidget.AddToViewport` _returnvalue 0))

(event `Key|LeftMouseButton`
  (params (Key :type "Key Structure"))
  (:`Pressed`
    (`GameplayStatics.PlayWorldCameraShake` "/Game/Gun/BP_CameraShake.BP_CameraShake_C" (`self.K2_GetActorLocation`) 0.0 100.0)
    (if (`.ReturnValue` (`PlayerController.GetHitResultUnderCursorByChannel` (`GameplayStatics.GetPlayerController` 0) "TraceTypeQuery1" true))
      _)))

(fn `UserConstructionScript`)